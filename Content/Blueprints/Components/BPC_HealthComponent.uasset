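; Actor component that tracks the owner's health and infection and mirrors both to the player HUD's health bar widget.
; Damage lowers health, healing raises it up to the maximum, and each infection hit adds a fixed step while shrinking maximum health.
; Empty health or full infection sends a death message to the owner, whose player reference also supplies the widget.
; Infection hits leave current health and its bar untouched.
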(event Custom|TakeDamage
  (params (Damage :type Float%20%28double-precision%29))
  (if (<= (- (Variables|Default|GetCurrentHealth) Damage) 0.0)
    (Variables|Default|SetCurrentHealth 0.0)
    (Default|SetHealth (Variables|Default|GetHealthWidgetRef) 0.0)
    (Class|BPIHelperHealthComponent|OnDeath(Message) (Components|GetOwner))
    (else
      (bind _output_get (Variables|Default|SetCurrentHealth (- (Variables|Default|GetCurrentHealth) Damage)))
      (Default|SetHealth (Variables|Default|GetHealthWidgetRef) (/ _output_get (Variables|Default|GetMaxHealth))))))

(event Custom|TakeInfection
  (if (>= (+ (Variables|Default|GetCurrentInfection) 1e+01) (Variables|Default|GetMaxInfection))
    (Variables|Default|SetCurrentInfection (Variables|Default|GetMaxInfection))
    (Default|SetInfection (Variables|Default|GetHealthWidgetRef) 1.0)
    (Class|BPIHelperHealthComponent|OnDeath(Message) (Components|GetOwner))
    (else
      (bind _output_get (Variables|Default|SetCurrentInfection (+ (Variables|Default|GetCurrentInfection) 1e+01)))
      (Variables|Default|SetMaxHealth (- (Variables|Default|GetMaxHealth) 1e+01))
      (Default|SetInfection (Variables|Default|GetHealthWidgetRef) (/ _output_get (Variables|Default|GetMaxInfection))))))

(event Custom|Heal
  (params (Amount :type Float%20%28double-precision%29))
  (bind _output_get (Variables|Default|SetCurrentHealth (Math|Float|Clamp(Float) (+ Amount (Variables|Default|GetCurrentHealth)) (Variables|Default|GetCurrentHealth) (Variables|Default|GetMaxHealth))))
  (Default|SetHealth (Variables|Default|GetHealthWidgetRef) (/ _output_get (Variables|Default|GetMaxHealth))))

(event EventBeginPlay
  (Variables|Default|SetCurrentHealth (Variables|Default|GetMaxHealth))
  (Variables|Default|SetCurrentInfection 0.0))

(event EventHealthBarWidgetRef
  (bind _player (Class|BPIHelperHealthComponent|RefPlayer(Message) (Components|GetOwner)))
  (Variables|Default|SetHealthWidgetRef (Variables|/Game/UI/BP_PlayerHUD.BP_PlayerHUD_C|GetHealthBarWidgetRef (Variables|/Game/Blueprints/Player/BP_Player.BP_Player_C|GetPlayerHUDRef _player)))
  (Default|SetHealth (Variables|Default|GetHealthWidgetRef) 1.0)
  (Default|SetInfection (Variables|Default|GetHealthWidgetRef) 0.0))

(fn RefPlayer
  (return 0))