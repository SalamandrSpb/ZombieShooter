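; Base weapon Blueprint for BP_Player that handles firing, magazine ammo, hand-socket attachment and HUD widget updates.
; WeaponFire plays the fire montage, spends a round, traces, then waits out FireRate, looping for one weapon type until stopped or empty.
; Traces run from the camera with random box spread, re-tracing from the muzzle when the aim point lies behind it.
; The end point is stored, with no damage applied here.
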(event Custom|WeaponFire
  (if (not (Variables|/Game/Blueprints/Player/BP_Player.BP_Player_C|GetIsStopFire (Variables|Default|GetPlayerRef))) :!label _label
    (Variables|FireWeapon|SetCanFire false)
    (Animation|Montage|PlayMontage (Variables|/Script/Engine.Character|GetMesh (Variables|Default|GetPlayerRef)) (Variables|AnimMontage|GetFireAnim)
      (:then
        (CallFunction|UpdateAmmoMagazine)
        (Default|UpdateAmmoInfo (Variables|UI|GetWeaponWidgetRef) (Variables|Ammo|GetAmmoMagazine) (Variables|Ammo|GetCurrentAmmo))
        (bind _hitresult (CallFunction|LineTraceLogic))
        (CallFunction|TraceEndPoint _hitresult)
        (Utilities|FlowControl|Delay (Variables|FireWeapon|GetFireRate))
        (if (Variables|Default|GetMagazineEmpty)
          (Variables|FireWeapon|SetCanFire false)
          (Development|PrintString "Кончились патроны")
          (else
            (Variables|FireWeapon|SetCanFire true)
            (if (Utilities|Enum|Equal(Enum) (Variables|Default|GetWeaponType) "NewEnumerator1")
              (goto _label))))))))

(event EventBeginPlay
  (bind _asbp_player (Utilities|Casting|CastToBP_Player (Components|GetOwner)))
  (Variables|Default|SetPlayerRef _asbp_player))

(fn ConstructionScript
  (Variables|Ammo|SetCurrentAmmo 48))

(fn AttachtoHand
  (params (HandSocket :type Name))
  (Transformation|AttachComponentToComponent (Variables|/Script/Engine.Character|GetMesh (Variables|Default|GetPlayerRef)) HandSocket "SnapToTarget" "SnapToTarget" "SnapToTarget" true))

(fn SetWeaponWidgetRef
  (params (WeaponWidget :type WBP%20Weapon%20Object%20Reference))
  (Variables|UI|SetWeaponWidgetRef WeaponWidget))

(fn UpdateWidgetInfo
  (Default|UpdateWeaponWidgetInfo (Variables|UI|GetWeaponWidgetRef) (Variables|Ammo|GetAmmoMagazine) (Variables|Ammo|GetCurrentAmmo) (Variables|UI|GetImageHud)))

(fn UpdateAmmoMagazine
  (bind _result (Math|Integer|DecrementInt (Variables|Ammo|GetAmmoMagazine))
    (:%20%20
      (if (== _result 0)
        (Variables|Default|SetMagazineEmpty true)))))

(fn LineTraceLogic
  (bind _returnvalue (Game|GetPlayerController 0))
  (bind _weaponmesh (Variables|Default|GetWeaponMesh))
  (bind _returnvalue_2 (Transformation|GetSocketLocation _weaponmesh "MuzzleFlash"))
  (bind (_location _rotation) (Pawn|GetPlayerViewPoint _returnvalue))
  (bind (_outhit _returnvalue_3) (Collision|LineTraceByChannel _location (Math|Random|RandomPointinBoundingBox (+ _location (* (Math|Rotator|GetRotationXVector _rotation) (Variables|FireWeapon|GetFireDistance))) (* "1.000000,1.000000,1.000000" (Variables|FireWeapon|GetSpread))) "TraceTypeQuery1" false 0 "ForDuration"))
  (if _returnvalue_3
    _
    (else
      _))
  (Variables|Default|SetHitResult _outhit)
  (if (> (Class|KismetMathLibrary|DegAcos (Math|Vector|DotProduct (Math|Vector|GetForwardVector (Transformation|GetSocketRotation (Variables|Default|GetWeaponMesh) "MuzzleFlash")) (- (Math|Vector|SelectVector (.ImpactPoint (Collision|BreakHitResult _outhit)) (.TraceEnd (Collision|BreakHitResult _outhit)) (.bBlockingHit (Collision|BreakHitResult _outhit))) (Transformation|GetSocketLocation (Variables|Default|GetWeaponMesh) "MuzzleFlash")))) 9e+01)
    (bind _outhit_2 (Collision|LineTraceByChannel _returnvalue_2 (Math|Random|RandomPointinBoundingBox (+ _returnvalue_2 (* (Math|Vector|GetForwardVector (Transformation|GetSocketRotation (Variables|Default|GetWeaponMesh) "MuzzleFlash")) (Variables|FireWeapon|GetFireDistance))) (* "1.000000,1.000000,1.000000" (Variables|FireWeapon|GetSpread))) "TraceTypeQuery1" false 0 "ForDuration"))
    (bind _output_get (Variables|Default|SetHitResult _outhit_2))
    (return _output_get)
    (else
      (return (Variables|Default|GetHitResult)))))

(fn TraceEndPoint
  (params (HitResult :type Hit%20Result%20Structure))
  (bind (_bblockinghit _binitialoverlap _time _distance _location _impactpoint _normal _impactnormal _physmat _hitactor _hitcomponent _hitbonename _bonename _hititem _elementindex _faceindex _tracestart _traceend) (Collision|BreakHitResult HitResult))
  (if _bblockinghit
    (Variables|Default|SetEndLineTrace _impactpoint)
    (else
      (Variables|Default|SetEndLineTrace _traceend))))